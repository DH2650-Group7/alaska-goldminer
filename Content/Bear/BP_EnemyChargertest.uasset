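; BP_EnemyChargertest is a test enemy that moves toward a ThirdPersonCharacter once PawnSensing sees it, using AI MoveTo.
; It also carries equipment and store functions, none invoked by its event graph.
; EquipItem attaches an item to the right-hand socket after UnequipItem detaches attached MiningEquipment and spawns its RespawnClass at the mesh.
; ToggleStore shows or removes the Store widget and mouse cursor, tracking state in a Pause flag.
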(event OnSeePawn(PawnSensing)
  (params (Pawn :type Pawn%20Object%20Reference))
  (bind _asthird_person_character (Utilities|Casting|CastToThirdPersonCharacter Pawn))
  (AI|AIMoveTo self "0, 0, 0" _asthird_person_character 5.0 false))

(fn ConstructionScript)

(fn EquipItem
  (params (Item :type Actor%20Object%20Reference))
  (CallFunction|UnequipItem)
  (bind _output_get (Variables|Default|SetEquippedItemReference Item))
  (Transformation|AttachComponentToComponent _output_get (Variables|Character|GetMesh) "RightHandSocket" "SnapToTarget" "SnapToTarget" "SnapToTarget" false)
  (Variables|Default|SetHasItemEquipped true))

(fn UnequipItem
  (Variables|Default|SetHasItemEquipped false)
  (for _array_element (Actor|GetAttachedActors)
    (Development|PrintString (Utilities|GetDisplayName _array_element))
    (bind _asmining_equipment (Utilities|Casting|CastToMiningEquipment _array_element))
    (bind _returnvalue (Game|SpawnActorfromClass (Variables|/Script/AlaskaGoldMiner.MiningEquipment|GetRespawnClass _asmining_equipment) (Math|Transform|MakeTransform "0, 0, 0" "0, 0,50.000000") "AdjustIfPossibleButAlwaysSpawn" 0 0))
    (Transformation|SetActorLocation _returnvalue (Transformation|GetWorldLocation (Variables|Character|GetMesh)) false false)
    (Transformation|DetachFromComponent (Variables|/Script/Engine.Actor|GetRootComponent _array_element) "KeepRelative" "KeepRelative" "KeepRelative" true)
    (Development|PrintString (Utilities|String|ToString(Object) _returnvalue))))

(fn ToggleStore
  (params (Char :type Third%20Person%20Character%20Object%20Reference))
  (bind _returnvalue (Game|GetPlayerController 0))
  (if (Variables|Default|GetPause)
    (Widget|RemovefromParent (Variables|Default|GetStore_Ref))
    (Variables|/Script/Engine.PlayerController|SetbShowMouseCursor _returnvalue false)
    (Variables|Default|SetStore_Ref 0)
    (Variables|Default|SetPause false)
    (else
      (Variables|Default|SetPause true)
      (Variables|/Script/Engine.PlayerController|SetbShowMouseCursor _returnvalue true)
      (bind _returnvalue_2 (UserInterface|CreateWidget "/Game/HUD_UI/Store.Store_C"))
      (bind _output_get (Variables|Default|SetStore_Ref _returnvalue_2))
      (UserInterface|Viewport|AddtoViewport _output_get 0))))