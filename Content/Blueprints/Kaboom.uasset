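; Kaboom is a Blueprint that blows apart a Stonehenge set of destructible pieces when E is pressed.
; A DoOnce gate limits the blast to one trigger, which switches on physics simulation for all the pieces and then fires impulses from multiple radial force components.
; It then loops over numbered components and spawns an actor at each one's world location, with the class not specified in the graph.
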(event Input|KeyboardEvents|E
  (params (Key :type Key%20Structure))
  (:Pressed
    (Utilities|FlowControl|DoOnce false
      (:Completed
        (Physics|SetSimulatePhysics (Variables|Default|Getstonehenge_DM1) true)
        (Class|RadialForceComponent|FireImpulse (Variables|Default|GetRadialForce))
        (for _array_element (Utilities|Array|MakeArray (Variables|Default|Get6) (Variables|Default|Get2) (Variables|Default|Get3) (Variables|Default|Get4) (Variables|Default|Get5) (Variables|Default|Get1) (Variables|Default|Get7) (Variables|Default|Get8) (Variables|Default|Get9) (Variables|Default|Get10))
          (Game|SpawnActorfromClass "/Game/StarterContent/Blueprints/Blueprint_Effect_Explosion.Blueprint_Effect_Explosion_C" (Math|Transform|MakeTransform (Transformation|GetWorldLocation _array_element) "0, 0, 0" "1.000000,1.000000,1.000000") "Undefined" 0 0))))))

(fn ConstructionScript)