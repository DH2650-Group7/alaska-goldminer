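; StoreBP is a world actor that lets the player toggle the store HUD while standing in its overlap area.
; It caches the AGMPlayerController on BeginPlay, then enables input and shows an "Open Store" hint when ThirdPersonCharacter overlaps, reversing both on exit.
; I, O and the gamepad top and right face buttons all call the controller's ToggleHUD with Store on release, with no separate open or close logic.
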(event Collision|EventActorBeginOverlap
  (params (OtherActor :type Actor%20Object%20Reference))
  (bind _pcref (Variables|Default|GetPCRef))
  (Utilities|Casting|CastToThirdPersonCharacter OtherActor)
  (Input|EnableInput _pcref)
  (Default|ShowHUDHint _pcref "I" "Y" "Open Store"))

(event Collision|EventActorEndOverlap
  (params (OtherActor :type Actor%20Object%20Reference))
  (bind _pcref (Variables|Default|GetPCRef))
  (Utilities|Casting|CastToThirdPersonCharacter OtherActor)
  (Input|DisableInput _pcref)
  (Default|HideHUDHint _pcref))

(event EventBeginPlay
  (bind _asagmplayer_controller (Utilities|Casting|CastToAGMPlayerController (Game|GetPlayerController 0)))
  (Variables|Default|SetPCRef _asagmplayer_controller))

(event Input|GamepadEvents|GamepadFaceButtonRight
  (params (Key :type Key%20Structure))
  (:Released
    (Default|ToggleHUD (Variables|Default|GetPCRef) "/Game/HUD_UI/Store/Store.Store_C")))

(event Input|KeyboardEvents|O
  (params (Key :type Key%20Structure))
  (:Released
    (Default|ToggleHUD (Variables|Default|GetPCRef) "/Game/HUD_UI/Store/Store.Store_C")))

(event Input|KeyboardEvents|I
  (params (Key :type Key%20Structure))
  (:Released
    (Default|ToggleHUD (Variables|Default|GetPCRef) "/Game/HUD_UI/Store/Store.Store_C")))

(event Input|GamepadEvents|GamepadFaceButtonTop
  (params (Key :type Key%20Structure))
  (:Released
    (Default|ToggleHUD (Variables|Default|GetPCRef) "/Game/HUD_UI/Store/Store.Store_C")))

(fn ConstructionScript)