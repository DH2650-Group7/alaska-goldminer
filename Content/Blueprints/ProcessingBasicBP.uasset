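; Interactable refinement table actor that lets the player open the Refinement HUD while standing near it.
; It caches the AGMPlayerController on BeginPlay, then overlap events enable or disable input on the actor and show or hide a key and gamepad hint.
; Releasing K or gamepad Y toggles the Refinement screen through the player controller.
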(event Collision|EventActorBeginOverlap
  (params (OtherActor :type Actor%20Object%20Reference))
  (bind _pcref (Variables|Default|GetPCRef))
  (Input|EnableInput _pcref)
  (Default|ShowHUDHint _pcref "K" "Y" "Use Refinement Table"))

(event Collision|EventActorEndOverlap
  (params (OtherActor :type Actor%20Object%20Reference))
  (bind _pcref (Variables|Default|GetPCRef))
  (Input|DisableInput _pcref)
  (Default|HideHUDHint _pcref))

(event EventBeginPlay
  (bind _asagmplayer_controller (Utilities|Casting|CastToAGMPlayerController (Game|GetPlayerController 0)))
  (Variables|Default|SetPCRef _asagmplayer_controller))

(event Input|GamepadEvents|GamepadFaceButtonTop
  (params (Key :type Key%20Structure))
  (:Released
    (bind _asagmplayer_controller (Utilities|Casting|CastToAGMPlayerController (Game|GetPlayerController 0)))
    (Default|ToggleHUD _asagmplayer_controller "/Game/HUD_UI/Refinement.Refinement_C")))

(event Input|KeyboardEvents|K
  (params (Key :type Key%20Structure))
  (:Released
    (bind _asagmplayer_controller (Utilities|Casting|CastToAGMPlayerController (Game|GetPlayerController 0)))
    (Default|ToggleHUD _asagmplayer_controller "/Game/HUD_UI/Refinement.Refinement_C")))

(fn ConstructionScript)