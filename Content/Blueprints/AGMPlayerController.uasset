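; Player controller that owns the game HUD and controls an on-screen key prompt for player actions.
; On BeginPlay it creates the GameHUD widget, stores a reference and adds it to the viewport.
; ShowHUDHint formats a "Press Key to Action" message and plays the EquipFadeIn animation, while HideHUDHint plays that animation in reverse.
; An unconnected leftover in ShowHUDHint for disabling input and clearing CanPickUp never runs.
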(event EventBeginPlay
  (bind _returnvalue (UserInterface|CreateWidget "/Game/HUD_UI/GameHUD.GameHUD_C" self))
  (bind _output_get (Variables|Default|SetHUD_Ref _returnvalue))
  (UserInterface|Viewport|AddtoViewport _output_get 0))

(fn ConstructionScript)

(fn ShowHUDHint
  (params (Key :type Text) (Action :type Text))
  (bind _hud_ref (Variables|Default|GetHUD_Ref))
  (Rendering|Components|TextRender|SetText (Variables|/Game/HUD_UI/GameHUD.GameHUD_C|GetHUDHint _hud_ref) (Utilities|Text|FormatText "Press {Key} to {Action}" Key Action))
  (UserInterface|Animation|PlayAnimation _hud_ref (Variables|/Game/HUD_UI/GameHUD.GameHUD_C|GetEquipFadeIn _hud_ref) 0.0 1 "Forward" 1.0))

(fn HideHUDHint
  (bind _hud_ref (Variables|Default|GetHUD_Ref))
  (UserInterface|Animation|PlayAnimation _hud_ref (Variables|/Game/HUD_UI/GameHUD.GameHUD_C|GetEquipFadeIn _hud_ref) 0.0 1 "Reverse" 1.0))