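; Game state that holds the ore inventory and a slowly regenerating Health value.
; Inventory functions count, add and remove ore in a map keyed by ore type, refusing over-removal with a printed warning.
; BeginPlay spawns a helper actor high above the origin for SlugOre and GoldChipOre, so RefinesInto can read that property by class.
; Tick uses a Delay to add Health about every half second while below full.
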(event EventTick
  (params (DeltaSeconds :type Float%20%28single-precision%29))
  (Utilities|FlowControl|Delay 0.5)
  (if (< (Variables|Default|GetHealth) 1.0)
    (Variables|Default|SetHealth (+ (Variables|Default|GetHealth) 0.01))))

(event EventBeginPlay
  (bind _returnvalue (Math|Transform|MakeTransform "0, 0,5000.000000" "0, 0, 0" "0.100000,0.100000,0.100000"))
  (bind _orehelpermap (Variables|Default|GetOreHelperMap))
  (bind _returnvalue_2 (Game|SpawnActorfromClass "/Game/Ore/SlugOre.SlugOre_C" _returnvalue "Undefined" 0 0))
  (bind _returnvalue_3 (Game|SpawnActorfromClass "/Game/Ore/GoldChipOre.GoldChipOre_C" _returnvalue "Undefined" 0 0))
  (Utilities|Map|Add _orehelpermap "/Game/Ore/SlugOre.SlugOre_C" _returnvalue_2)
  (Utilities|Map|Add _orehelpermap "/Game/Ore/GoldChipOre.GoldChipOre_C" _returnvalue_3))

(fn ConstructionScript)

(fn GetOreCount
  (params (Ore :type Ore%20Class%20Reference))
  (bind _oreinventory (Variables|Default|GetOreInventory))
  (bind (_value _returnvalue) (Utilities|Map|Find _oreinventory Ore))
  (if _returnvalue
    (return _value)
    (else
      (return 0))))

(fn ObtainOre
  (params (Ore :type Ore%20Class%20Reference) (Quantity :type Integer))
  (bind _oreinventory (Variables|Default|GetOreInventory))
  (bind (_value _returnvalue) (Utilities|Map|Find _oreinventory Ore))
  (if _returnvalue
    (Utilities|Map|Add _oreinventory Ore (+ Quantity _value))
    (else
      (Utilities|Map|Add _oreinventory Ore Quantity))))

(fn RefinesInto
  (params (Ore :type Ore%20Class%20Reference))
  (return (Variables|/Script/AlaskaGoldMiner.Ore|GetRefinesInto (.Value (Utilities|Map|Find (Variables|Default|GetOreHelperMap) Ore)))))

(fn RemoveOre
  (params (Ore :type Ore%20Class%20Reference) (Quantity :type Integer))
  (bind _oreinventory (Variables|Default|GetOreInventory))
  (bind _value (Utilities|Map|Find _oreinventory Ore))
  (if (> Quantity _value)
    (Development|PrintString "You're trying to remove more ore than you have" true true "(R=1.000000,G=0.135502,B=0.000000,A=1.000000)")
    (else
      (Utilities|Map|Add (Variables|Default|GetOreInventory) Ore (- _value Quantity)))))