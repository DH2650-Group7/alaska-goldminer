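; Shopkeeper actor that greets the player and opens the store when the player is nearby.
; Front overlap plays a greeting sound and salute animation before returning to idle, while Top overlap plays an easter-egg sound, each throttled by a DoOnce reset after delays.
; Actor overlap enables input and shows a HUD hint, so releasing I calls ToggleStore on the ThirdPersonCharacter; leaving disables input and hides the hint.
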(event OnComponentBeginOverlap(Top)
  (params (OverlappedComponent :type Primitive%20Component%20Object%20Reference) (OtherActor :type Actor%20Object%20Reference) (OtherComp :type Primitive%20Component%20Object%20Reference) (OtherBodyIndex :type Integer) (bFromSweep :type Boolean) (SweepResult :type Hit%20Result%20Structure%20%28by%20ref%29))
  (Utilities|FlowControl|DoOnce false :!label _label
    (:Completed
      (Audio|PlaySoundatLocation "/Game/StarterContent/Audio/ShopEasterEgg.ShopEasterEgg" (Transformation|GetWorldLocation (Variables|SkeletalMeshActor|GetSkeletalMeshComponent)) "0, 0, 0" 1.0 1.0 0.0 0 0 0)
      (Utilities|FlowControl|Delay 4.0)
      (goto _label Reset))))

(event OnComponentEndOverlap(Top)
  (params (OverlappedComponent :type Primitive%20Component%20Object%20Reference) (OtherActor :type Actor%20Object%20Reference) (OtherComp :type Primitive%20Component%20Object%20Reference) (OtherBodyIndex :type Integer)))

(event OnComponentBeginOverlap(Front)
  (params (OverlappedComponent :type Primitive%20Component%20Object%20Reference) (OtherActor :type Actor%20Object%20Reference) (OtherComp :type Primitive%20Component%20Object%20Reference) (OtherBodyIndex :type Integer) (bFromSweep :type Boolean) (SweepResult :type Hit%20Result%20Structure%20%28by%20ref%29))
  (bind _skeletalmeshcomponent (Variables|SkeletalMeshActor|GetSkeletalMeshComponent))
  ;[1 1 1] VL + Animation
  (Utilities|FlowControl|DoOnce false :!label _label
    (:Completed
      (Audio|PlaySoundatLocation "/Game/StarterContent/Audio/ShopGreeting.ShopGreeting" (Transformation|GetWorldLocation _skeletalmeshcomponent) "0, 0, 0" 1.0 1.0 0.0 0 0 0)
      (Components|Animation|PlayAnimation _skeletalmeshcomponent "/Game/Shopkeeper/Salute.Salute" false)
      (Utilities|FlowControl|Delay 3.0)
      (Components|Animation|PlayAnimation _skeletalmeshcomponent "/Game/Shopkeeper/Idle.Idle" true)
      (Utilities|FlowControl|Delay 1.0)
      (goto _label Reset))))

(event Collision|EventActorBeginOverlap
  (params (OtherActor :type Actor%20Object%20Reference))
  (bind _pcref (Variables|Default|GetPCRef))
  ;[1 1 1] StoreBP
  (Input|EnableInput _pcref)
  (Default|ShowHUDHint _pcref "I" "Open Store"))

(event Collision|EventActorEndOverlap
  (params (OtherActor :type Actor%20Object%20Reference))
  (bind _pcref (Variables|Default|GetPCRef))
  ;[1 1 1] StoreBP
  (Input|DisableInput _pcref)
  (Default|HideHUDHint _pcref))

(event EventBeginPlay
  ;[1 1 1] StoreBP
  (bind _asagmplayer_controller (Utilities|Casting|CastToAGMPlayerController (Game|GetPlayerController 0)))
  (Variables|Default|SetPCRef _asagmplayer_controller))

(event Input|KeyboardEvents|I
  (params (Key :type Key%20Structure))
  ;[1 1 1] StoreBP
  (:Released
    (bind _asthird_person_character (Utilities|Casting|CastToThirdPersonCharacter (Game|GetPlayerCharacter 0)))
    (Default|ToggleStore _asthird_person_character)))

(fn ConstructionScript)